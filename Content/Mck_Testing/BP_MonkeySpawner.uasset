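; BP_MonkeySpawner spawns a batch of endangered monkeys at target points when SpawnEndangeredMonkeys is called, with the batch size capped per lap.
; BeginPlay shuffles the instance-set target points once.
; A fast looping timer spawns one monkey per tick with random yaw, removing each used point so later batches draw from those remaining.
; The timer clears and the count resets once MaxMonkeysPerLap is reached.
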(event Custom|SpawnMonkey
  (Game|SpawnActorfromClass "/Game/Mck_Testing/BP_EndangeredMonkey.BP_EndangeredMonkey_C" (Math|Transform|MakeTransform (Transformation|GetActorLocation (Utilities|Array|Get(acopy) (Variables|Default|GetTargetPoints))) (Math|Rotator|MakeRotator 0.0 0.0 (.yaw (Math|Random|RandomRotator false))) "1.000000,1.000000,1.000000") "AlwaysSpawn" "MultiplyWithRoot" 0 0)
  (Utilities|Array|RemoveIndex (Variables|Default|GetTargetPoints))
  (bind _result (Math|Integer|IncrementInt (Variables|Default|GetCurrentMonkeys))
    (:%20%20
      (if (>= _result (Variables|Default|GetMaxMonkeysPerLap))
        (Utilities|Time|ClearandInvalidateTimerbyHandle (Variables|Default|GetMonkeyTimerHandle))
        (Variables|Default|SetCurrentMonkeys 0)))))

(event EventBeginPlay
  (Utilities|Array|Shuffle (Variables|Default|GetTargetPoints)))

(event EventSpawnEndangeredMonkeys
  (bind _returnvalue (Utilities|Time|SetTimerbyEvent (delegate Custom|SpawnMonkey) 0.1 true))
  (Variables|Default|SetMonkeyTimerHandle _returnvalue))

(fn ConstructionScript)