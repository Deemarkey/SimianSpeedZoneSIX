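; BP_EndangeredMonkey is a hittable monkey actor that costs the player points when BP_MonkeyPawn runs into it.
; On BeginPlay it sets its sphere to overlap pawns and picks one of six random colour materials for the mesh.
; Any overlap plays hit sounds and knocks the mesh along the player's forward vector with physics.
; Only a BP_MonkeyPawn overlap then triggers the delayed HUD point loss and later self-destruction.
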(event OnComponentBeginOverlap(Sphere1)
  (params (OverlappedComponent :type Primitive%20Component%20Object%20Reference) (OtherActor :type Actor%20Object%20Reference) (OtherComp :type Primitive%20Component%20Object%20Reference) (OtherBodyIndex :type Integer) (bFromSweep :type Boolean) (SweepResult :type Hit%20Result%20Structure%20%28by%20ref%29))
  (bind _staticmesh (Variables|Default|GetStaticMesh))
  (Audio|PlaySound2D "/Game/Assets/SFX/Thud.Thud" 1.0 1.0 0.0 0 0)
  (Audio|PlaySound2D "/Game/Assets/SFX/MonkeyHit.MonkeyHit" 1.0 1.0 0.0 0 0)
  (Physics|SetSimulatePhysics _staticmesh true)
  (Physics|AddImpulse _staticmesh (Transformation|GetActorForwardVector (Game|Player|GetPlayerPawn 0)) "None" false)
  (bind _asbp_monkey_pawn (Utilities|Casting|CastToBP_MonkeyPawn OtherActor))
  (Utilities|FlowControl|Delay 1.0)
  (Default|LosePoints (Variables|/Game/Player/BP_MonkeyPawn.BP_MonkeyPawn_C|GetReference_HUD _asbp_monkey_pawn))
  (Utilities|FlowControl|Delay 5.0)
  (Actor|DestroyActor))

(event EventBeginPlay
  (Collision|SetCollisionResponsetoChannel (Variables|Default|GetSphere1) "ECC_Pawn" "ECR_Overlap")
  (Rendering|Material|SetMaterial (Variables|Default|GetStaticMesh) 0 (Utilities|Select :Index (Math|Random|RandomIntegerinRange 0 5) :Option%200 "/Game/Assets/GradientMaterials/MI_red.MI_red" :Option%201 "/Game/Assets/GradientMaterials/MI_Yellow.MI_Yellow" :Option%202 "/Game/Assets/GradientMaterials/MI_Orange.MI_Orange" :Option%203 "/Game/Assets/GradientMaterials/MI_Blue1.MI_Blue1" :Option%204 "/Game/Assets/GradientMaterials/MI_Green.MI_Green" :Option%205 "/Game/Assets/GradientMaterials/MI_Purple.MI_Purple")))

(fn ConstructionScript)