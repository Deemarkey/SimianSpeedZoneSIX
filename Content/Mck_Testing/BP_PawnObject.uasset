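; Player pawn for a spline-track game: it auto-travels the track, steers sideways and reloads the level on a hit.
; A Timeline moves the actor along SplineToFollow, restarting faster after each pass by shortening TimeToComplete, with no lower limit.
; Enhanced Input adjusts TurningAlpha, which Tick turns into clamped lateral offset and mesh yaw, alongside debug prints.
; A looping timer, randomized once, spawns BP_Obstacle "bananas" at the mesh.
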(event Custom|Hit
  (bind _returnvalue (Game|GetCurrentLevelName true))
  (Game|OpenLevel(byName) (Utilities|String|StringToName _returnvalue)))

(event Custom|Move%20Actor
  (Components|Timeline|SetPlayRate (Variables|Default|GetTimeline) (/ 1.0 (Variables|Default|GetTimeToComplete)))
  (bind _newtrack_0 (Timeline|Timeline Play)
    (:Update
      (Transformation|SetActorLocationAndRotation (Spline|GetLocationatDistanceAlongSpline (Variables|/Game/Mck_Testing/BP_SplinePath.BP_SplinePath_C|GetSpline (Variables|Default|GetSplineToFollow)) (Math|Float|Lerp 0.0 (Spline|GetSplineLength (Variables|/Game/Mck_Testing/BP_SplinePath.BP_SplinePath_C|GetSpline (Variables|Default|GetSplineToFollow))) _newtrack_0) "World") (Spline|GetRotationatDistanceAlongSpline (Variables|/Game/Mck_Testing/BP_SplinePath.BP_SplinePath_C|GetSpline (Variables|Default|GetSplineToFollow)) (Math|Float|Lerp 0.0 (Spline|GetSplineLength (Variables|/Game/Mck_Testing/BP_SplinePath.BP_SplinePath_C|GetSpline (Variables|Default|GetSplineToFollow))) _newtrack_0) "World")))
    (:Finished
      (bind _output_get (Variables|Default|SetTimeToComplete (- (Variables|Default|GetTimeToComplete) 2.0)))
      (Components|Timeline|SetPlayRate (Variables|Default|GetTimeline) (/ 1.0 _output_get))
      (Timeline|Timeline PlayFromStart))))

(event Custom|Spawn%20Banana
  (bind _staticmesh (Variables|Default|GetStaticMesh))
  (bind _returnvalue (Transformation|GetWorldLocation _staticmesh))
  (Game|SpawnActorfromClass "/Game/Mck_Testing/BP_Obstacle.BP_Obstacle_C" (Math|Transform|MakeTransform (Math|Vector|MakeVector (.x _returnvalue) (.y _returnvalue) (.z _returnvalue)) "0, 0, 0" "1.200000,2.000000,2.000000") "Undefined" "MultiplyWithRoot" 0 0))

(event Input|EnhancedActionEvents|EnhancedInputActionLeft_IA
  (params (ActionValue :type Boolean) (ElapsedSeconds :type Float%20%28double-precision%29) (TriggeredSeconds :type Float%20%28double-precision%29) (InputAction :type Input%20Action%20Object%20Reference :default "/Game/Left_IA.Left_IA"))
  (if (not (== (Variables|Default|GetHorizontalMovement) (* (Variables|Default|GetTrackWidth) -1.0)))
    (Variables|Default|SetTurningAlpha (- (Variables|Default|GetTurningAlpha) (Variables|Default|GetTurnSpeed)))))

(event Input|EnhancedActionEvents|EnhancedInputActionRight_IA
  (params (ActionValue :type Boolean) (ElapsedSeconds :type Float%20%28double-precision%29) (TriggeredSeconds :type Float%20%28double-precision%29) (InputAction :type Input%20Action%20Object%20Reference :default "/Game/Right_IA.Right_IA"))
  (if (not (== (Variables|Default|GetHorizontalMovement) (Variables|Default|GetTrackWidth)))
    (Variables|Default|SetTurningAlpha (+ (Variables|Default|GetTurningAlpha) (Variables|Default|GetTurnSpeed)))))

(event EventBeginPlay
  (bind _asplayer_controller (Utilities|Casting|CastToPlayer_Controller (Pawn|GetController)))
  (Input|AddMappingContext (PlayerController|LocalPlayerSubsystems|GetEnhancedInputLocalPlayerSubsystem _asplayer_controller) "/Game/MONKE/MAGENTAIMCC.MAGENTAIMCC" 0 "(bIgnoreAllPressedKeysUntilRelease=True,bForceImmediately=False,bNotifyUserSettings=False)")
  (CallFunction|MoveActor)
  (Utilities|Time|SetTimerbyFunctionName 0 "Spawn Banana" (Math|Random|RandomFloatinRange 1.0 3.0) true))

(event EventTick
  (params (DeltaSeconds :type Float%20%28single-precision%29))
  ;[0.15 0.15 0.15 0.5] Debug
  (Development|PrintString (Utilities|String|Append "Horizontal Movement: " (Utilities|String|ToString(Float) (Variables|Default|GetHorizontalMovement))) true true "(R=0.000000,G=0.660000,B=1.000000,A=1.000000)" 0.0)
  (Development|PrintString (Utilities|String|Append "Turning Alpha: " (Utilities|String|ToString(Float) (Variables|Default|GetTurningAlpha))) true true "(R=0.000000,G=0.660000,B=1.000000,A=1.000000)" 0.0)
  (Development|PrintString (Utilities|String|Append "TimeToComplete: " (Utilities|String|ToString(Float) (Variables|Default|GetTimeToComplete))) true true "(R=0.000000,G=0.660000,B=1.000000,A=1.000000)" 0.0)
  (Variables|Default|SetHorizontalMovement (Math|Float|Clamp(Float) (- (Variables|Default|GetHorizontalMovement) (Math|Float|Lerp 0.0 -1e+01 (Variables|Default|GetTurningAlpha))) (* (Variables|Default|GetTrackWidth) -1.0) (Variables|Default|GetTrackWidth)))
  (Transformation|SetRelativeLocation (Variables|Default|GetScene) (Math|Vector|MakeVector 0.0 (Variables|Default|GetHorizontalMovement) 0.0) false false)
  (Transformation|SetRelativeRotation (Variables|Default|GetStaticMesh) (Math|Rotator|MakeRotator 0.0 0.0 (Math|Float|Lerp 0.0 25.0 (Variables|Default|GetTurningAlpha))) false false)
  (if (or (== (Variables|Default|GetHorizontalMovement) (* (Variables|Default|GetTrackWidth) -1.0)) (== (Variables|Default|GetHorizontalMovement) (Variables|Default|GetTrackWidth)))
    (Variables|Default|SetTurningAlpha 0.0)))

(fn ConstructionScript)