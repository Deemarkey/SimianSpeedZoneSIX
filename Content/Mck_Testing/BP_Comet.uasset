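; BP_Comet is a short-lived comet hazard that damages the monkey pawn on contact.
; On BeginPlay it sets a lifespan, randomizes the Scene component's rotation and runs a brief looping timer that steps up its scale, so it grows in after spawning.
; When its Box component begins overlapping a BP_MonkeyPawn, it sends a fixed damage amount through DamageMessage.
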(event OnComponentBeginOverlap(Box)
  (params (OverlappedComponent :type Primitive%20Component%20Object%20Reference) (OtherActor :type Actor%20Object%20Reference) (OtherComp :type Primitive%20Component%20Object%20Reference) (OtherBodyIndex :type Integer) (bFromSweep :type Boolean) (SweepResult :type Hit%20Result%20Structure%20%28by%20ref%29))
  (bind _asbp_monkey_pawn (Utilities|Casting|CastToBP_MonkeyPawn OtherActor))
  (Class|DamageBPI|Damage(Message) _asbp_monkey_pawn 3.0))

(event Custom|Grow
  (bind _scene (Variables|Default|GetScene))
  (Transformation|SetRelativeScale3D _scene (+ (Variables|/Script/Engine.SceneComponent|GetRelativeScale3D _scene) 0.1)))

(event EventBeginPlay
  (Actor|SetLifeSpan 1e+01)
  (Transformation|SetRelativeRotation (Variables|Default|GetScene) (Math|Rotator|MakeRotator (Math|Random|RandomFloatinRange 0.0 1.8e+02) (Math|Random|RandomFloatinRange 0.0 1.8e+02) (Math|Random|RandomFloatinRange 0.0 1.8e+02)) false false)
  (bind _returnvalue (Utilities|Time|SetTimerbyFunctionName 0 "Grow" 0.05 true))
  (Utilities|FlowControl|Delay 0.5)
  (Utilities|Time|ClearandInvalidateTimerbyHandle _returnvalue))

(fn ConstructionScript)