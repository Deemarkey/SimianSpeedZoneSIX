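; Icicle spawner that places one BP_Icicle at a random target point each time SpawnIcicles is triggered.
; BeginPlay shuffles the TargetPoints array, and each spawn uses then removes the first entry, so points do not repeat.
; Icicles spawn with the RotationForPlayerDetect rotation, then only their HitBox receives a random world yaw.
; SpawnIcicles has no empty-array check and no caller within this Blueprint.
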(event EventBeginPlay
  (Utilities|Array|Shuffle (Variables|Default|GetTargetPoints)))

(event EventSpawnIcicles
  (bind _returnvalue (Game|SpawnActorfromClass "/Game/PaulTesting/Icicle/BP_Icicle.BP_Icicle_C" (Math|Transform|MakeTransform (Transformation|GetActorLocation (Utilities|Array|Get(acopy) (Variables|Default|GetTargetPoints))) (Variables|Default|GetRotationForPlayerDetect) "1.000000,1.000000,1.000000") "AlwaysSpawn" "MultiplyWithRoot" 0 0))
  (bind _output_get (Variables|Default|SetIcicle _returnvalue))
  (Transformation|SetWorldRotation (Variables|/Game/PaulTesting/Icicle/BP_Icicle.BP_Icicle_C|GetHitBox _output_get) (Math|Rotator|MakeRotator 0.0 0.0 (.yaw (Math|Random|RandomRotator false))) false false)
  (Utilities|Array|RemoveIndex (Variables|Default|GetTargetPoints)))

(fn ConstructionScript)