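; BP_PaintableFloor is a floor actor prototype for painting into a render target where the camera looks.
; BeginPlay clears the render target, then Tick line-traces from the camera location toward its forward vector times a distance, without adding the start location.
; Tick opens the render target canvas, but the polygon draw at the hit's collision UV and the closing call are unwired, so nothing gets painted.
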(event EventTick
  (params (DeltaSeconds :type Float%20%28single-precision%29))
  (bind _returnvalue (Game|GetPlayerController 0))
  (bind _playercameramanager (Variables|/Script/Engine.PlayerController|GetPlayerCameraManager _returnvalue))
  (bind _outhit (Collision|LineTraceByChannel (Camera|GetCameraLocation _playercameramanager) (* (Math|Vector|GetForwardVector (Variables|/Script/Engine.PlayerCameraManager|GetTransformComponent _playercameramanager)) (Variables|Default|GetLineTraceDistance)) "TraceTypeQuery1" false 0 "None" false))
  (bind (_canvas _size _context) (Rendering|BeginDrawCanvastoRenderTarget (Variables|Default|GetPaintRenderTarget))))

(event EventBeginPlay
  (bind _paintrendertarget (Variables|Default|GetPaintRenderTarget))
  (Rendering|ClearRenderTarget2D _paintrendertarget (Variables|/Script/Engine.TextureRenderTarget2D|GetClearColor _paintrendertarget)))

(fn ConstructionScript)