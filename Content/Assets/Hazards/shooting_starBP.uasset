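; Shooting star hazard actor that moves back and forth along a path set by three point components.
; BeginPlay caches their world locations and starts the Movement timeline, whose Movement track blends X from Point1 to Point2 while its Bottom track blends Z from Point2 to Point3.
; Y keeps the actor's current value.
; When the timeline finishes, a FlipFlop alternates between reversing and playing it, looping the motion.
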(event Custom|Playfromend
  (bind (_direction _movement _bottom) (Timeline|Movement Reverse)
    (:Update
      (Transformation|SetActorLocation (Math|Vector|MakeVector (.x (Math|Vector|Lerp(Vector) (Variables|Default|GetP1Location) (Variables|Default|GetP2Location) _movement)) (.y (Transformation|GetActorLocation)) (Math|Float|Lerp (.z (Variables|Default|GetP2Location)) (.z (Variables|Default|GetP3location)) _bottom)) false false))
    (:Finished
      (Utilities|FlowControl|FlipFlop
        (:A
          (CallFunction|Playfromend))
        (:B
          (CallFunction|Playfromstart))))))

(event Custom|Playfromstart
  (bind (_direction _movement _bottom) (Timeline|Movement Play)
    (:Update
      (Transformation|SetActorLocation (Math|Vector|MakeVector (.x (Math|Vector|Lerp(Vector) (Variables|Default|GetP1Location) (Variables|Default|GetP2Location) _movement)) (.y (Transformation|GetActorLocation)) (Math|Float|Lerp (.z (Variables|Default|GetP2Location)) (.z (Variables|Default|GetP3location)) _bottom)) false false))
    (:Finished
      (Utilities|FlowControl|FlipFlop
        (:A
          (CallFunction|Playfromend))
        (:B
          (CallFunction|Playfromstart))))))

(event EventBeginPlay
  (Variables|Default|SetP1Location (Transformation|GetWorldLocation (Variables|Default|Getpoint%201)))
  (Variables|Default|SetP2Location (Transformation|GetWorldLocation (Variables|Default|Getpoint%202)))
  (Variables|Default|SetP3location (Transformation|GetWorldLocation (Variables|Default|Getpoint%203)))
  (bind (_direction _movement _bottom) (Timeline|Movement Play)
    (:Update
      (Transformation|SetActorLocation (Math|Vector|MakeVector (.x (Math|Vector|Lerp(Vector) (Variables|Default|GetP1Location) (Variables|Default|GetP2Location) _movement)) (.y (Transformation|GetActorLocation)) (Math|Float|Lerp (.z (Variables|Default|GetP2Location)) (.z (Variables|Default|GetP3location)) _bottom)) false false))
    (:Finished
      (Utilities|FlowControl|FlipFlop
        (:A
          (CallFunction|Playfromend))
        (:B
          (CallFunction|Playfromstart))))))

(fn ConstructionScript)