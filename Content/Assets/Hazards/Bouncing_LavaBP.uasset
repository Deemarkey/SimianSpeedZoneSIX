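; Bouncing lava hazard that damages the monkey pawn on overlap and expires after a fixed lifespan set at BeginPlay.
; Each hit applies a velocity-change impulse to the Star component at the actor's location, kicking it upward with random sideways X motion.
; Overlap casts to BP_MonkeyPawn and sends DamageMessage before a self-resetting DoOnce, so that one-second gate does not throttle damage.
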(event EventBeginPlay
  (Actor|SetLifeSpan 14.0))

(event Collision|EventActorBeginOverlap
  (params (OtherActor :type Actor%20Object%20Reference))
  ;[0.15 0.15 0.15 0.5] Hit Player
  (bind _asbp_monkey_pawn (Utilities|Casting|CastToBP_MonkeyPawn OtherActor))
  (Class|DamageBPI|Damage(Message) _asbp_monkey_pawn 1.0)
  (Utilities|FlowControl|DoOnce false :!label _label
    (:Completed
      (Utilities|FlowControl|Delay 1.0)
      (goto _label Reset))))

(event Collision|EventHit
  (params (MyComp :type Primitive%20Component%20Object%20Reference) (Other :type Actor%20Object%20Reference) (OtherComp :type Primitive%20Component%20Object%20Reference) (bSelfMoved :type Boolean) (HitLocation :type Vector :default "0, 0, 0") (HitNormal :type Vector :default "0, 0, 0") (NormalImpulse :type Vector :default "0, 0, 0") (Hit :type Hit%20Result%20Structure%20%28by%20ref%29))
  ;[0.15 0.15 0.15 0.5] spawns lava at location and impulses
  (Class|PrimitiveComponent|AddVelocityChangeImpulseatLocation (Variables|Default|Getstar) (Math|Vector|MakeVector (Math|Random|RandomFloatinRange -5e+02 5e+02) 0.0 5e+02) (Transformation|GetActorLocation) "None"))

(fn ConstructionScript)