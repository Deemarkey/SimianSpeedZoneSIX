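; Player monkey pawn for a lap-based obstacle dodger, auto-moving along a spline while the player steers sideways.
; Possession sets up HUD, save data, character mesh and input, then starts movement, banana spawning and icicles.
; A timeline drives spline travel, shortening each lap and triggering a slow-motion jet cinematic; Tick applies clamped lateral offset and eased lean.
; Damage leads to death, which spins the monkey, stops movement, saves records and shows the death screen.
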(event Custom|monkeydead
  (bind _newtrack_0 (Timeline|Timeline Stop)
    (:Update
      (Transformation|SetActorLocationAndRotation (Spline|GetLocationatDistanceAlongSpline (Variables|/Game/Mck_Testing/BP_SplinePath.BP_SplinePath_C|GetSpline (Variables|References|GetReference_Spline)) (Math|Float|Lerp 0.0 (Spline|GetSplineLength (Variables|/Game/Mck_Testing/BP_SplinePath.BP_SplinePath_C|GetSpline (Variables|References|GetReference_Spline))) _newtrack_0) "World") (Spline|GetRotationatDistanceAlongSpline (Variables|/Game/Mck_Testing/BP_SplinePath.BP_SplinePath_C|GetSpline (Variables|References|GetReference_Spline)) (Math|Float|Lerp 0.0 (Spline|GetSplineLength (Variables|/Game/Mck_Testing/BP_SplinePath.BP_SplinePath_C|GetSpline (Variables|References|GetReference_Spline))) _newtrack_0) "World")))
    (:Finished
      (Variables|Default|SetLapsCompleted (+ (Variables|Default|GetLapsCompleted) 1))
      (Default|NewLap (Variables|References|GetReference_HUD))
      (bind _output_get (Variables|Default|SetTimeToComplete (- (Variables|Default|GetTimeToComplete) 2.0)))
      (Class|BPISpawnObstacles|SpawnIcicles(Message) (Variables|References|GetReference_IcicleSpawner))
      (Components|Timeline|SetPlayRate (Variables|Default|GetTimeline) (/ 1.0 _output_get))
      (Timeline|Timeline PlayFromStart))
    (:Cinematic%20Border
      (Default|PlayCinematicBorders (Variables|References|GetReference_HUD))
      (Utilities|FlowControl|Delay 4.0)
      (Default|SpawnJets (Variables|References|GetReference_JetSpawner))
      (Utilities|Time|SetGlobalTimeDilation 0.5)
      (Utilities|FlowControl|Delay 1.0)
      (Utilities|Time|SetGlobalTimeDilation 1.0)
      (Default|ClearBorders (Variables|References|GetReference_HUD)))))

(event Custom|Move%20Actor
  (Components|Timeline|SetPlayRate (Variables|Default|GetTimeline) (/ 1.0 (Variables|Default|GetTimeToComplete)))
  (Utilities|FlowControl|Sequence
    (:then_0
      (bind _newtrack_0 (Timeline|Timeline SetNewTime)
        (:Update
          (Transformation|SetActorLocationAndRotation (Spline|GetLocationatDistanceAlongSpline (Variables|/Game/Mck_Testing/BP_SplinePath.BP_SplinePath_C|GetSpline (Variables|References|GetReference_Spline)) (Math|Float|Lerp 0.0 (Spline|GetSplineLength (Variables|/Game/Mck_Testing/BP_SplinePath.BP_SplinePath_C|GetSpline (Variables|References|GetReference_Spline))) _newtrack_0) "World") (Spline|GetRotationatDistanceAlongSpline (Variables|/Game/Mck_Testing/BP_SplinePath.BP_SplinePath_C|GetSpline (Variables|References|GetReference_Spline)) (Math|Float|Lerp 0.0 (Spline|GetSplineLength (Variables|/Game/Mck_Testing/BP_SplinePath.BP_SplinePath_C|GetSpline (Variables|References|GetReference_Spline))) _newtrack_0) "World")))
        (:Finished
          (Variables|Default|SetLapsCompleted (+ (Variables|Default|GetLapsCompleted) 1))
          (Default|NewLap (Variables|References|GetReference_HUD))
          (bind _output_get (Variables|Default|SetTimeToComplete (- (Variables|Default|GetTimeToComplete) 2.0)))
          (Class|BPISpawnObstacles|SpawnIcicles(Message) (Variables|References|GetReference_IcicleSpawner))
          (Components|Timeline|SetPlayRate (Variables|Default|GetTimeline) (/ 1.0 _output_get))
          (Timeline|Timeline PlayFromStart))
        (:Cinematic%20Border
          (Default|PlayCinematicBorders (Variables|References|GetReference_HUD))
          (Utilities|FlowControl|Delay 4.0)
          (Default|SpawnJets (Variables|References|GetReference_JetSpawner))
          (Utilities|Time|SetGlobalTimeDilation 0.5)
          (Utilities|FlowControl|Delay 1.0)
          (Utilities|Time|SetGlobalTimeDilation 1.0)
          (Default|ClearBorders (Variables|References|GetReference_HUD)))))
    (:then_1
      (Timeline|Timeline Play))))

(event Custom|Spawn%20Banana
  (if (Variables|Default|GetisDead)
    (Utilities|Time|ClearandInvalidateTimerbyHandle (stale EventPossessed _returnvalue_4))
    (else
      (Game|SpawnActorfromClass "/Game/Mck_Testing/BP_Obstacle.BP_Obstacle_C" (Math|Transform|MakeTransform (Transformation|GetWorldLocation (Variables|Default|GetBananaSpawnPoint)) "0, 0, 0" "1.000000,1.000000,1.000000") "Undefined" "MultiplyWithRoot" 0 0))))

(event Custom|Death
  ;[0.15 0 0.003493 0.5] Death
  (if (<= (Variables|Default|GetHealth) 0.0)
    (Variables|Default|SetisDead true)
    (Input|SetInputModeUIOnly (Game|GetPlayerController 0) 0 "DoNotLock" false)
    (CallFunction|Spinning)
    (CallFunction|Monkeydead)
    (CallFunction|SaveGame)
    (bind _returnvalue (UserInterface|CreateWidget "/Game/UI/WB_DeathScreen.WB_DeathScreen_C"))
    (UserInterface|Viewport|AddtoViewport _returnvalue 0)
    (Variables|/Script/Engine.PlayerController|SetbShowMouseCursor (Game|GetPlayerController 0) true)
    (Widget|RemovefromParent (Variables|References|GetReference_HUD))))

(event Custom|SpinOut
  ;[0.002496 0.15 0 0.5] Spinning Monkeys
  (Utilities|FlowControl|Delay 1.0)
  (Variables|Default|SetisSpinning false)
  (bind _rotation (Timeline|spin Stop)
    (:Update
      (Transformation|SetRelativeRotation (Variables|Default|GetStaticMesh) (Math|Rotator|Lerp(Rotator) "0, 0, 0" "0.000000,360.000000,0.000000" _rotation) false false)
      (CallFunction|SpinOut))))

(event Custom|Spinning
  ;[0.002496 0.15 0 0.5] Spinning Monkeys
  (Variables|Default|SetisSpinning true)
  (bind _rotation (Timeline|spin PlayFromStart)
    (:Update
      (Transformation|SetRelativeRotation (Variables|Default|GetStaticMesh) (Math|Rotator|Lerp(Rotator) "0, 0, 0" "0.000000,360.000000,0.000000" _rotation) false false)
      (CallFunction|SpinOut))))

(event Input|EnhancedActionEvents|EnhancedInputActionIA_Look
  (params (ActionValue :type Vector%202D%20Structure) (ElapsedSeconds :type Float%20%28double-precision%29) (TriggeredSeconds :type Float%20%28double-precision%29) (InputAction :type Input%20Action%20Object%20Reference :default "/Game/Player/Inputs/IA_Look.IA_Look"))
  (bind _sensitivity (Variables|Default|GetSensitivity))
  (Pawn|Input|AddControllerYawInput (* (.x ActionValue) _sensitivity))
  (Pawn|Input|AddControllerPitchInput (* _sensitivity (.y ActionValue))))

(event Input|EnhancedActionEvents|EnhancedInputActionIA_SteerLeft
  (params (ActionValue :type Boolean) (ElapsedSeconds :type Float%20%28double-precision%29) (TriggeredSeconds :type Float%20%28double-precision%29) (InputAction :type Input%20Action%20Object%20Reference :default "/Game/Player/Inputs/IA_SteerLeft.IA_SteerLeft"))
  (:Triggered
    (if (not (Variables|Default|GetisSpinning))
      (if (not (== (Variables|Default|GetHorizontalMovement) (* (Variables|Default|GetTrackWidth) -1.0)))
        (Variables|Default|SetIsSteering true)
        (Variables|Default|SetTurningAlpha (Math|Float|Clamp(Float) (- (Variables|Default|GetTurningAlpha) (Variables|Default|GetTurnSpeed)) -1.5 1.5)))))
  (:Completed
    (Variables|Default|SetIsSteering false)))

(event Input|EnhancedActionEvents|EnhancedInputActionIA_SteerRight
  (params (ActionValue :type Boolean) (ElapsedSeconds :type Float%20%28double-precision%29) (TriggeredSeconds :type Float%20%28double-precision%29) (InputAction :type Input%20Action%20Object%20Reference :default "/Game/Player/Inputs/IA_SteerRight.IA_SteerRight"))
  (:Triggered
    (if (not (Variables|Default|GetisSpinning))
      (if (not (== (Variables|Default|GetHorizontalMovement) (Variables|Default|GetTrackWidth)))
        (Variables|Default|SetIsSteering true)
        (Variables|Default|SetTurningAlpha (Math|Float|Clamp(Float) (+ (Variables|Default|GetTurningAlpha) (Variables|Default|GetTurnSpeed)) -1.5 1.5)))))
  (:Completed
    (Variables|Default|SetIsSteering false)))

(event Input|EnhancedActionEvents|EnhancedInputActionIA_Pause
  (params (ActionValue :type Boolean) (ElapsedSeconds :type Float%20%28double-precision%29) (TriggeredSeconds :type Float%20%28double-precision%29) (InputAction :type Input%20Action%20Object%20Reference :default "/Game/Player/Inputs/IA_Pause.IA_Pause"))
  (:Started
    (CallFunction|PauseGame)))

(event EventTick
  (params (DeltaSeconds :type Float%20%28single-precision%29))
  ;[0.15 0 0 0.5] Bad Monkey :(
  (if (not (Variables|Default|GetisSpinning))
    (Variables|Default|SetHorizontalMovement (Math|Float|Clamp(Float) (- (Variables|Default|GetHorizontalMovement) (Math|Float|Lerp 0.0 (Variables|Default|GetHorizontalSpeed) (Variables|Default|GetTurningAlpha))) (* (Variables|Default|GetTrackWidth) -1.0) (Variables|Default|GetTrackWidth)))
    (Transformation|SetRelativeLocation (Variables|Default|GetScene) (Math|Vector|MakeVector 0.0 (Variables|Default|GetHorizontalMovement) 0.0) false false)
    (Transformation|SetRelativeRotation (Variables|Default|GetStaticMesh) (Math|Rotator|MakeRotator (Math|Float|Lerp 0.0 25.0 (Variables|Default|GetTurningAlpha)) 0.0 (Math|Float|Lerp 0.0 1e+01 (Variables|Default|GetTurningAlpha))) false false)
    (if (Variables|Default|GetIsSteering)
      (if (or (== (Variables|Default|GetHorizontalMovement) (* (Variables|Default|GetTrackWidth) -1.0)) (== (Variables|Default|GetHorizontalMovement) (Variables|Default|GetTrackWidth))) :!label _label
        (Variables|Default|SetTurningAlpha 0.0 :!label _label_2))
      (elif (> (Variables|Default|GetTurningAlpha) 0.0)
        (Variables|Default|SetTurningAlpha (- (Variables|Default|GetTurningAlpha) (Variables|Default|GetTurnSpeed)))
        (if (Math|Float|NearlyEqual(Float) (Variables|Default|GetTurningAlpha) 0.0 0.1) :!label _label_3
          (goto _label_2)
          (else
            (goto _label)))
        (elif (< (Variables|Default|GetTurningAlpha) 0.0)
          (Variables|Default|SetTurningAlpha (+ (Variables|Default|GetTurningAlpha) (Variables|Default|GetTurnSpeed)))
          (goto _label_3))))))

(event EventDamage
  (params (Damage :type Float%20%28double-precision%29))
  ;[0.15 0.15 0.15 0.5] Damage
  (bind _output_get (Variables|Default|SetHealth (- (Variables|Default|GetHealth) Damage)))
  (Development|PrintString (Utilities|String|ToString(Float) _output_get))
  (CallFunction|Death))

(event EventPossessed
  (params (NewController :type Controller%20Object%20Reference))
  (bind _returnvalue (Game|GetPlayerController 0))
  (Input|SetInputModeGameOnly _returnvalue false)
  (Variables|/Script/Engine.PlayerController|SetbShowMouseCursor _returnvalue false)
  (bind _returnvalue_2 (UserInterface|CreateWidget "/Game/UI/WB_HUD.WB_HUD_C"))
  (bind _output_get (Variables|References|SetReference_HUD _returnvalue_2))
  (UserInterface|Viewport|AddtoViewport _output_get 0)
  (bind _returnvalue_3 (SaveGame|DoesSaveGameExist "Save1"))
  (if _returnvalue_3
    (CallFunction|Loadgame)
    (else
      (CallFunction|SaveGame)))
  (Variables|Default|SetisDead false)
  (Default|EventCountdown (Variables|References|GetReference_HUD))
  (CallFunction|Characterselect)
  (bind _asmonkey_player_controller (Utilities|Casting|CastToMonkey_PlayerController (Game|GetPlayerController 0)))
  (Input|AddMappingContext (PlayerController|LocalPlayerSubsystems|GetEnhancedInputLocalPlayerSubsystem _asmonkey_player_controller) "/Game/Player/Inputs/IMC_Monkey.IMC_Monkey" 0 "(bIgnoreAllPressedKeysUntilRelease=True,bForceImmediately=False,bNotifyUserSettings=False)")
  (Utilities|FlowControl|Delay 3.0)
  (CallFunction|MoveActor)
  (bind _returnvalue_4 (Utilities|Time|SetTimerbyFunctionName 0 "Spawn Banana" (Math|Random|RandomFloatinRange 1.0 3.0) true))
  (bind _outactors (Actor|GetAllActorsOfClass "/Game/PaulTesting/Icicle/BP_IcicleSpawner.BP_IcicleSpawner_C"))
  (for _array_element _outactors
    (if (Utilities|DoesObjectImplementInterface _array_element "/Game/PaulTesting/Icicle/BPI_SpawnObstacles.BPI_SpawnObstacles_C")
      (bind _output_get_2 (Variables|References|SetReference_IcicleSpawner _array_element))
      (Class|BPISpawnObstacles|SpawnIcicles(Message) _output_get_2))))

(fn ConstructionScript)

(fn Characterselect
  (Components|StaticMesh|SetStaticMesh (Variables|Default|GetStaticMesh) (Utilities|Select :Index (Variables|Default|GetSelection) :NewEnumerator0 "/Game/MONKE/SM_RonaldRedFixed.SM_RonaldRedFixed" :NewEnumerator1 "/Game/MONKE/SM_GeraldGreenFixed.SM_GeraldGreenFixed" :NewEnumerator2 "/Game/MONKE/SM_MagentaMarkFixed.SM_MagentaMarkFixed" :NewEnumerator3 "/Game/MONKE/SM_SpectreOrangeFixed.SM_SpectreOrangeFixed")))

(fn SaveGame
  (bind _returnvalue (SaveGame|CreateSaveGameObject "/Game/Player/SG_SaveData.SG_SaveData_C"))
  (bind _output_get (Variables|Default|SetScore (Variables|/Game/UI/WB_HUD.WB_HUD_C|GetTimeFloat (Variables|References|GetReference_HUD))))
  (if (> _output_get (Variables|Default|GetHighscore))
    (bind _output_get_2 (Variables|Default|SetHighscore (Variables|Default|GetScore)))
    (Variables|/Game/Player/SG_SaveData.SG_SaveData_C|SetHighScore _returnvalue _output_get_2)
    (if (> (Variables|Default|GetLapsCompleted) (Variables|Default|GetHighestLap))
      (bind _output_get_3 (Variables|Default|SetHighestLap (Variables|Default|GetLapsCompleted)))
      (Variables|/Game/Player/SG_SaveData.SG_SaveData_C|SetHighestLap _returnvalue _output_get_3)
      (SaveGame|SaveGametoSlot _returnvalue "Save1"))))

(fn Loadgame
  (bind _returnvalue (SaveGame|LoadGamefromSlot "Save1"))
  (bind _assave_data_bp (Utilities|Casting|CastToSG_SaveData _returnvalue))
  (bind _output_get (Variables|Default|SetAs%20Save%20Data%20BP _assave_data_bp))
  (Variables|Default|SetHighestLap (Variables|/Game/Player/SG_SaveData.SG_SaveData_C|GetHighestLap _output_get))
  (Variables|Default|SetHighscore (Variables|/Game/Player/SG_SaveData.SG_SaveData_C|GetHighScore _output_get))
  (SaveGame|SaveGametoSlot _returnvalue "Save1"))

(fn PauseGame
  (bind _returnvalue (Game|GetPlayerController 0))
  (Game|SetGamePaused true)
  (Input|SetInputModeUIOnly _returnvalue 0 "DoNotLock" false)
  (Variables|/Script/Engine.PlayerController|SetbShowMouseCursor _returnvalue true)
  (bind _returnvalue_2 (UserInterface|CreateWidget "/Game/UI/WB_PauseMenu.WB_PauseMenu_C" 0 self))
  (bind _output_get (Variables|References|SetReference_PauseMenu _returnvalue_2))
  (UserInterface|Viewport|AddtoViewport _output_get 0))

(fn UnPauseGame
  (bind _returnvalue (Game|GetPlayerController 0))
  (Game|SetGamePaused false)
  (Widget|RemovefromParent (Variables|References|GetReference_PauseMenu))
  (Input|SetInputModeGameOnly _returnvalue true)
  (Variables|/Script/Engine.PlayerController|SetbShowMouseCursor _returnvalue false))